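; BP_Player is the player shape that must match walls by lane position, size and color, with FMOD sounds on each change.
; Arrow keys step through preset locations and size meshes, A/Z/E/R swap color materials, and Escape opens L_Main.
; CheckRule compares a wall's two type indices and color to the player's state, incrementing the HUD counter on a match.
; BeginPlay adds input mapping, creates HUD and pause widgets once started, and caches wall DataTable rows.
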(event `self.ReceiveBeginPlay`
  (bind _returnvalue (`GameplayStatics.GetPlayerController` 0))
  (bind _asgi_game_instance (cast `/Game/GI_GameInstance` (`GameplayStatics.GetGameInstance`)))
  (set `self.As GI Game Instance` _asgi_game_instance)
  (`EnhancedInputSubsystemInterface.AddMappingContext` (pcsubsystem `EnhancedInputLocalPlayerSubsystem` (`GameplayStatics.GetPlayerController` 0)) "/Game/InputManager/IAM.IAM" 0 (struct))
  (`|ExecutionSequence`
    (:`then_0`
      (if (`/Game/GI_GameInstance.IsGameStarted` (`self.As GI Game Instance`))
        (bind _returnvalue_2 (`|CreateWidget` "/Game/UI/UI_HUD.UI_HUD_C" _returnvalue))
        (bind _output_get (set `self.HUD` _returnvalue_2))
        (`UserWidget.AddToViewport` _output_get 0)
        (bind _returnvalue_3 (`|CreateWidget` "/Game/UI/UI_PauseMenu.UI_PauseMenu_C" _returnvalue))
        (set `self.HUD_Pause` _returnvalue_3)))
    (:`then_1`
      (bind _outrownames (`DataTableFunctionLibrary.GetDataTableRowNames` "/Game/Actors/Walls/Datas/DT_WallReferences.DT_WallReferences"))
      (for _array_element _outrownames
        (bind _returnvalue_4 (`|GetDataTableRow` "/Game/Actors/Walls/Datas/DT_WallReferences.DT_WallReferences" _array_element)
          (:`then`
            (`KismetArrayLibrary.Array_AddUnique` (`self.Out Row`) _returnvalue_4)))))))

(event `Key|Down`
  (params (Key :type "Key Structure"))
  (bind _currentindex (`self.CurrentIndex`))
  (:`Pressed`
    (if (not (== _currentindex 0))
      (bind _output_get (set `self.CurrentIndex` (+ _currentindex -1)))
      (for (_array_element _array_index) (`self.MeshSizeList`)
        (if (== _output_get _array_index)
          (set `SkeletalMeshComponent.SkeletalMeshAsset` _array_element (`self.Mesh`))
          ;[0.5312 0.01737 0.4256 0.5] FMOD
          (`FMODBlueprintStatics.PlayEventAttached` "/Game/FMOD/Events/SFX/SFX_ScaleChange.SFX_ScaleChange" (`self.CapsuleComponent`) "None" (0.0 0.0 0.0) "KeepRelativeOffset" :!label _label))))))

(event `Key|Up`
  (params (Key :type "Key Structure"))
  (bind _currentindex (`self.CurrentIndex`))
  (:`Pressed`
    (if (not (== _currentindex 4))
      (bind _output_get (set `self.CurrentIndex` (+ _currentindex 1)))
      (for (_array_element _array_index) (`self.MeshSizeList`)
        (if (== _output_get _array_index)
          (set `SkeletalMeshComponent.SkeletalMeshAsset` _array_element (`self.Mesh`))
          (goto _label))))))

(event `Key|Left`
  (params (Key :type "Key Structure"))
  (:`Pressed`
    (for (_array_element _array_index) (`self.PosList`)
      (if (== _array_index (+ (`self.CurrentIndexPos`) -1))
        (set `self.CurrentIndexPos` _array_index)
        (`self.K2_SetActorLocation` _array_element false true)
        (`|ExecutionSequence`
          (:`then_0`
            (break))
          (:`then_1`
            ;[0.5312 0.01737 0.4256 0.5] FMOD
            (`FMODBlueprintStatics.PlayEventAttached` "/Game/FMOD/Events/SFX/SFX_PlacementChange.SFX_PlacementChange" (`self.CapsuleComponent`) "None" (0.0 0.0 0.0) "KeepRelativeOffset" :!label _label_2)))))))

(event `Key|Right`
  (params (Key :type "Key Structure"))
  (:`Pressed`
    (for (_array_element _array_index) (`self.PosList`)
      (if (== _array_index (+ (`self.CurrentIndexPos`) 1))
        (set `self.CurrentIndexPos` _array_index)
        (`self.K2_SetActorLocation` _array_element false true)
        (`|ExecutionSequence`
          (:`then_0`
            (goto _label_2))
          (:`then_1`
            (break)))))))

(event `Key|A`
  (params (Key :type "Key Structure"))
  (:`Pressed`
    (`PrimitiveComponent.SetMaterial` (`self.Mesh`) 0 "/Game/Art/Materials/Main_Object/M_Main_Object_Red.M_Main_Object_Red")
    ;[0.5312 0.01737 0.4256 0.5] FMOD
    (`FMODBlueprintStatics.PlayEventAttached` "/Game/FMOD/Events/SFX/SFX_ColorChange.SFX_ColorChange" (`self.CapsuleComponent`) "None" (0.0 0.0 0.0) "KeepRelativeOffset" :!label _label_3)))

(event `Key|Z`
  (params (Key :type "Key Structure"))
  (:`Pressed`
    (`PrimitiveComponent.SetMaterial` (`self.Mesh`) 0 "/Game/Art/Materials/Main_Object/M_Main_Object_Green.M_Main_Object_Green")
    (goto _label_3)))

(event `Key|E`
  (params (Key :type "Key Structure"))
  (:`Pressed`
    (`PrimitiveComponent.SetMaterial` (`self.Mesh`) 0 "/Game/Art/Materials/Main_Object/M_Main_Object_Yellow.M_Main_Object_Yellow")
    (goto _label_3)))

(event `Key|R`
  (params (Key :type "Key Structure"))
  (:`Pressed`
    (`PrimitiveComponent.SetMaterial` (`self.Mesh`) 0 "/Game/Art/Materials/Main_Object/M_Main_Object_Blue.M_Main_Object_Blue")
    (goto _label_3)))

(event `Key|Escape`
  (params (Key :type "Key Structure"))
  (:`Pressed`
    (`GameplayStatics.OpenLevel` "L_Main")))

(fn `CheckRule`
  (params (HWallType :type Integer) (VWallType :type Integer) (TextStaticMesh :type "StaticMesh Object Reference") (ColorsMaterialMesh :type "Material Object Reference"))
  (returns (ValidRules :type Boolean))
  (bind _actualsize (`/Game/UI/UI_HUD.ActualSize` (`self.HUD`)))
  (bind (_keypin _valuepin) (`|MapForEach` (`self.ColorMeshType`))
    (:`then`
      (if (== (`PrimitiveComponent.GetMaterial` (`self.Mesh`) 0) _keypin)
        (if (and (== HWallType (`self.CurrentIndexPos`)) (== VWallType (`self.CurrentIndex`)) (== (`KismetStringLibrary.Conv_StringToName` (`KismetSystemLibrary.GetObjectName` ColorsMaterialMesh)) (`KismetStringLibrary.Conv_StringToName` (`KismetStringLibrary.Conv_NameToString` _valuepin))))
          (`TextBlock.SetText` _actualsize (`KismetTextLibrary.Conv_IntToText` (+ (`KismetStringLibrary.Conv_StringToInt` (`KismetTextLibrary.Conv_TextToString` (`TextBlock.Text` _actualsize))) 1)))
          (return true)
          (else
            (return false)))))))

(fn `UserConstructionScript`)