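; BP_Wall is a moving obstacle with a Stroop-style color word that tests the player on overlap.
; Init matches GM wall data for mesh and types, picks a random DT_StroopData word mesh and valid color material, then moves along -X on Tick.
; The player's CheckRule decides the outcome: success dissolves the wall via a timeline-driven material with Niagara and FMOD effects, while failure stops all walls and triggers death.
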(event `Init`
  (params (MeshIndex :type Integer) (Speed :type "Float (double-precision)"))
  (bind _asgm (cast `/Game/GM` (`GameplayStatics.GetGameMode`)))
  (bind _output_get (set `self.As GM` _asgm))
  (bind _outrownames (`DataTableFunctionLibrary.GetDataTableRowNames` "/Game/Actors/Walls/Datas/DT_StroopData.DT_StroopData"))
  (bind _returnvalue (`|GetDataTableRow` "/Game/Actors/Walls/Datas/DT_StroopData.DT_StroopData" (`KismetArrayLibrary.Array_Random` _outrownames))
    (:`then`
      (for _array_element (`/Game/GM.WallRef` _output_get)
        (bind (_targetwallmesh _targetcolormesh) (break `/Game/Actors/Walls/Datas/S_WallData` (`|GetArrayItem` (`/Game/GM.WallsData` _output_get) MeshIndex)))
        (if (== (`|GetEnumeratorName` (`.WallType_2_DEE4541146A59D53E20912ABD9FA08BF` (break `/Game/Actors/Walls/Datas/S_ReferenceTable` _array_element))) (`|GetEnumeratorName` _targetwallmesh))
          (bind (_colorstaticmesh _colorlistvalid) (break `/Game/Actors/Walls/Datas/S_ColorReferences` _returnvalue))
          (set `self.CurrentMesh` _colorstaticmesh)
          (set `self.CurrentMaterial Colors` (`KismetArrayLibrary.Array_Random` _colorlistvalid))
          (set `self.TargetColorMesh` _targetcolormesh)
          (bind _asbp_player (cast `/Game/Player/BP_Player` (`GameplayStatics.GetPlayerCharacter` 0)))
          (set `self.As BP Player` _asbp_player)
          (`self.ProcessData` _array_element)
          (bind _result (`self.Setup` MeshIndex))
          (if _result
            (`self.Move` Speed)))))))

(event `self.ReceiveTick`
  (params (DeltaSeconds :type "Float (single-precision)"))
  (if (`self.CanMove`)
    (`self.K2_AddActorWorldOffset` (* (* (`KismetMathLibrary.MakeVector` -1.0) (`self.Speed`)) DeltaSeconds) true)))

(event `self.MeshCollider.OnComponentBeginOverlap`
  (params (OverlappedComponent :type "PrimitiveComponent Object Reference") (OtherActor :type "Actor Object Reference") (OtherComp :type "PrimitiveComponent Object Reference") (OtherBodyIndex :type Integer) (bFromSweep :type Boolean) (SweepResult :type "HitResult Structure (by ref)"))
  (bind _asbp_player (cast `/Game/Player/BP_Player` OtherActor))
  (bind _validrules (`/Game/Player/BP_Player.CheckRule` _asbp_player (`self.HType`) (`self.VType`) null (`self.CurrentMaterial Colors`)))
  (if _validrules
    (`self.SetCanMove` false)
    (bind _returnvalue (`PrimitiveComponent.CreateDynamicMaterialInstance` (`self.Mesh`) 0 "/Game/Fx_DissolveWall.Fx_DissolveWall" "None"))
    (set `self.DisolveMaterialInstance` _returnvalue)
    (bind _returnvalue_2 (`NiagaraFunctionLibrary.SpawnSystemAtLocation` (`BlueprintMapLibrary.Map_Find` (`self.Fxmap`) (`self.TargetColorMesh`)) (`SceneComponent.K2_GetComponentLocation` (`Actor.RootComponent` (`GameplayStatics.GetPlayerPawn` 0)))))
    (`FMODBlueprintStatics.PlayEventAtLocation` "/Game/FMOD/Events/SFX/SFX_Sparks.SFX_Sparks" (`KismetMathLibrary.MakeTransform` (`SceneComponent.K2_GetComponentLocation` _returnvalue_2)))
    (`self.Death`)
    (`KismetSystemLibrary.PrintText` "Destroy")
    (`self.OnSuccess`)
    (else
      (`self.SetCanMove` false true)
      (`self.OnDeath`)
      ;[0.5312 0.01737 0.4256 0.5] FMOD
      (bind _asgi_game_instance (cast `/Game/GI_GameInstance` (`GameplayStatics.GetGameInstance`)))
      (`FMODBlueprintStatics.EventInstanceSetParameter` (`/Game/GI_GameInstance.FmodEventInstance` _asgi_game_instance) "PlayerState" 2.0)
      (`FMODBlueprintStatics.PlayEvent2D` "/Game/FMOD/Events/SFX/SFX_Death.SFX_Death"))))

(event `Death`
  (if (`KismetSystemLibrary.IsValid` (`self.DisolveMaterialInstance`))
    (bind (_direction _alpha) (`Timeline|Timeline` :!label _label)
      (:`Update`
        (`MaterialInstanceDynamic.SetScalarParameterValue` (`self.DisolveMaterialInstance`) "Dissolve" _alpha))
      (:`Finished`
        (`self.K2_DestroyActor`)))
    (else
      (bind _returnvalue (`PrimitiveComponent.CreateDynamicMaterialInstance` (`self.Mesh`) 0 "/Game/Fx_DissolveWall.Fx_DissolveWall" "None"))
      (set `self.DisolveMaterialInstance` _returnvalue)
      (goto _label :!via `PlayFromStart`))))

(fn `Move`
  (params (Speed :type "Float (double-precision)"))
  (set `self.Speed` Speed)
  (set `self.CanMove` true))

(fn `ProcessData`
  (params (WallData :type "/Game/Actors/Walls/Datas/S_ReferenceTable Structure"))
  (bind (_walltype _horizontaltype _verticaltype) (break `/Game/Actors/Walls/Datas/S_ReferenceTable` WallData))
  (set `self.VType` _verticaltype)
  (set `self.HType` (`KismetMathLibrary.Conv_ByteToInt` (cast `/Game/Actors/Walls/Datas/E_HorizontalTypes` _horizontaltype))))

(fn `SetCanMove`
  (params (ValueStatus :type Boolean) (AllWall :type Boolean))
  (if AllWall
    (bind _outactors (`GameplayStatics.GetAllActorsOfClass` "BP_Wall_C"))
    (for _array_element _outactors
      (set `/Game/Actors/Walls/BP_Wall.CanMove` ValueStatus _array_element))
    (else
      (set `self.CanMove` ValueStatus))))

(fn `Setup`
  (params (MeshIndex :type Integer))
  (returns (Result :type Boolean))
  (bind _colorstext (`self.ColorsText`))
  (bind _asgm (cast `/Game/GM` (`GameplayStatics.GetGameMode`))
    (:`then`
      (bind _result (`/Game/GM.GetDataAtRowIndex` _asgm MeshIndex))
      (`|ExecutionSequence`
        (:`then_0`
          (bind _result_2 (`/Game/GM.GetTargetMeshForIndex` _asgm (`.TargetWallMesh_23_90F4C1784F8F65431876E6A648CF05F7` (break `/Game/Actors/Walls/Datas/S_WallData` _result))))
          (bind _returnvalue (`StaticMeshComponent.SetStaticMesh` (`self.Mesh`) _result_2))
          (bind _output_get (set `self.Status` _returnvalue))
          (if (not _output_get)
            (return false)))
        (:`then_1`
          (`StaticMeshComponent.SetStaticMesh` _colorstext (`self.CurrentMesh`))
          (`PrimitiveComponent.SetMaterial` _colorstext 0 (`self.CurrentMaterial Colors`)))
        (:`then_4`
          (return (`self.Status`)))))
    (:`CastFailed`
      (`KismetSystemLibrary.PrintText` "Unable to get GM on BP_Wall" true true (struct :`R` 1.0 :`A` 1.0)))))

(fn `UserConstructionScript`)