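; Spawn point actor that launches the sequence of moving BP_Wall obstacles and handles the outcome of each.
; InitSpawn reads the wall count from the GM game mode and starts a looping timer that spawns indexed walls, then opens UI_PauseMenu once all are spawned.
; Wall success and death events forward to ACGroundController; death also destroys all walls, then pauses into the menu after a delay.
; Dissolve material instances are created, but their Timeline is unconnected.
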(event `InitSpawn`
  (bind _returnvalue (`KismetMaterialLibrary.CreateDynamicMaterialInstance` "/Game/Art/Materials/Fx/Fx_Dissolve.Fx_Dissolve"))
  (set `self.ObjectMatInst` _returnvalue)
  (bind _returnvalue_2 (`KismetMaterialLibrary.CreateDynamicMaterialInstance` "/Game/Fx_DissolveWall.Fx_DissolveWall"))
  (set `self.WallMatInst` _returnvalue_2)
  (bind _asgm (cast `/Game/GM` (`GameplayStatics.GetGameMode`))
    (:`then`
      (set `self.TotalWallCount` (`KismetArrayLibrary.Array_Length` (`/Game/GM.WallsData` _asgm)))
      (`KismetSystemLibrary.K2_SetTimerDelegate` (delegate `SpawnWall`) (* 2.56 (`self.DelayBetweenWalls`)) true))
    (:`CastFailed`
      (`KismetSystemLibrary.PrintText` "Unable to get the GameMode from spawn point" true true (struct :`R` 1.0 :`B` 0.000183 :`A` 1.0)))))

(event `SpawnWall`
  (bind _spawnedwallcount (`self.SpawnedWallCount`))
  (if (< (`self.SpawnedWallCount`) (`self.TotalWallCount`))
    (bind _returnvalue (`|SpawnActorFromClass` "/Game/Actors/Walls/BP_Wall.BP_Wall_C" (`self.GetTransform`) "Undefined" "MultiplyWithRoot" null null))
    (if (`KismetSystemLibrary.IsValid` _returnvalue)
      (`/Game/Actors/Walls/BP_Wall.Init` _returnvalue _spawnedwallcount 600.0)
      (`/Engine/EditorBlueprintResources/StandardMacros.IncrementInt` _spawnedwallcount
        (:`  `
          (add `/Game/Actors/Walls/BP_Wall.OnDeath` _returnvalue (delegate `Death`))
          (add `/Game/Actors/Walls/BP_Wall.OnSuccess` _returnvalue (delegate `Success`))))
      (else
        (`KismetSystemLibrary.PrintText` "Unable to spawn wall" true true (struct :`R` 1.0 :`G` 0.041261 :`A` 1.0))))
    (else
      (`WidgetLayoutLibrary.RemoveAllWidgets`)
      (bind _returnvalue_2 (`|CreateWidget` "/Game/UI/UI_PauseMenu.UI_PauseMenu_C" (`GameplayStatics.GetPlayerController` 0)))
      (`UserWidget.AddToViewport` _returnvalue_2 0))))

(event `Success`
  (`/Game/GroundShader/ACGroundController.Success` (`self.ACGroundController`)))

(event `Death`
  (bind _returnvalue (`GameplayStatics.GetPlayerController` 0))
  (`/Game/GroundShader/ACGroundController.Death` (`self.ACGroundController`))
  (bind _outactors (`GameplayStatics.GetAllActorsOfClass` "/Game/Actors/Walls/BP_Wall.BP_Wall_C"))
  (for _array_element _outactors
    (`self.K2_DestroyActor` _array_element))
  (`KismetSystemLibrary.Delay` 3.0)
  (`GameplayStatics.SetGamePaused` true)
  (bind _returnvalue_2 (`|CreateWidget` "/Game/UI/UI_PauseMenu.UI_PauseMenu_C" _returnvalue))
  (`UserWidget.AddToViewport` _returnvalue_2 0)
  (set `PlayerController.bShowMouseCursor` true _returnvalue))

(fn `UserConstructionScript`)